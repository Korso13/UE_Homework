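; BP_BML is an interactable missile launcher that sends its missile mesh straight up when used.
; Interact starts the visual and audio effects, sets the launched flag only if both are valid, and reports the interaction finished either way.
; While launched, Tick calls FlyMissile, which raises the mesh a fixed step per frame, independent of delta time, then hides it and disables its collision at a height limit.
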(event EventBeginPlay)

(event Collision|EventActorBeginOverlap
  (params (OtherActor :type Actor%20Object%20Reference)))

(event EventTick
  (params (DeltaSeconds :type Float%20%28single-precision%29))
  (if (Variables|Default|GetIsLaunched)
    (CallFunction|FlyMissile)))

(event EventInteract
  (params (Instigator :type Actor%20Object%20Reference))
  (Variables|Default|SetInteractionInstigator Instigator)
  (bind _visual_sfx (Variables|Default|GetVisual%20SFX)
    (:then
      (Components|Activation|Activate _visual_sfx false)
      (bind _audio_sfx (Variables|Default|GetAudio%20SFX)
        (:then
          (Audio|Components|Audio|Play _audio_sfx 0.0)
          (Variables|Default|SetIsLaunched true)
          (Class|BaseInteractionActor|OnInteractionFinished (Variables|Default|GetInteractionInstigator)))
        (:else
          (Class|BaseInteractionActor|OnInteractionFinished (Variables|Default|GetInteractionInstigator) :!label _label))))
    (:else
      (goto _label))))

(fn ConstructionScript)

(fn FlyMissile
  (bind _missile_mesh (Variables|Default|GetMissile%20mesh))
  (bind _returnvalue (Transformation|GetWorldLocation _missile_mesh))
  (bind _missile_mesh_2 (Variables|Default|GetMissile%20mesh)
    (:then
      ;[0 0.2132 1] Checking if missile went too high
      (if (< (.z (Transformation|GetWorldLocation _missile_mesh_2)) 5e+03)
        ;[1 0.8857 0] Sending missile higher
        (Transformation|SetWorldLocation _missile_mesh (Math|Vector|MakeVector (.x _returnvalue) (.y _returnvalue) (+ (.z (Transformation|GetWorldLocation _missile_mesh_2)) 25.0)) false false)
        (else
          ;[1 0.07097 0.09003] Removing missile
          (Collision|SetCollisionEnabled (Variables|Default|GetMissile%20mesh) "NoCollision")
          (Rendering|SetVisibility (Variables|Default|GetMissile%20mesh) false false))))
    (:else)))