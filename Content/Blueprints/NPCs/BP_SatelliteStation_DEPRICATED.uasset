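; Deprecated satellite station Blueprint that acts as a quest giver, handing out quests from a list one at a time.
; BeginPlay pops the first entry of the Quests array into AvailableQuest.
; On Interact, it attaches that quest actor to the instigator, prints a greeting and the description, calls TakeQuest, then loads the next quest.
; Each interaction ends through OnInteractionFinished, with a printed notice when no quests remain.
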(event EventBeginPlay
  ;[1 0 0.7362] Obtainign a copy of first quest if there is one
  (if (Utilities|Array|IsValidIndex (Variables|Default|GetQuests))
    (Variables|Default|SetAvailableQuest (Utilities|Array|Get(acopy) (Variables|Default|GetQuests)))
    ;[1 0 0.06701] Removing first quest from array
    (Utilities|Array|RemoveIndex (Variables|Default|GetQuests))))

(event Collision|EventActorBeginOverlap
  (params (OtherActor :type Actor%20Object%20Reference)))

(event EventTick
  (params (DeltaSeconds :type Float%20%28single-precision%29)))

(event EventInteract
  (params (Instigator :type Actor%20Object%20Reference))
  (bind _quests (Variables|Default|GetQuests))
  ;[1 0 0.8549] Recording Quest requester
  (Variables|Default|SetQuest_Instigator Instigator)
  ;[1 0.2412 0.4976] Checking if there is a quest available. Ending interaction if not
  (bind _availablequest (Variables|Default|GetAvailableQuest)
    (:then
      ;[0 1 0.2464] Giving quest to quest requester
      (Transformation|AttachActorToActor _availablequest (Variables|Default|GetQuest_Instigator) "None" "SnapToTarget" "SnapToTarget" "SnapToTarget" true)
      (Development|PrintString (Utilities|String|Append "Hello,  " (Utilities|GetDisplayName (Variables|Default|GetQuest_Instigator)) "! Here is your mission!") true true "(R=0.000000,G=0.660000,B=1.000000,A=1.000000)" 3.0)
      (Development|PrintString (Utilities|String|ToString(Text) (Variables|/Script/QuestSystem.Quest|GetQuestDescription (Variables|Default|GetAvailableQuest))) true true "(R=0.000000,G=1.000000,B=0.172531,A=1.000000)" 7.0)
      (Class|Quest|TakeQuest (Variables|Default|GetAvailableQuest) (Variables|Default|GetQuest_Instigator))
      ;[1 0 0.7362] Obtaining a copy of the next quest if there is one
      (if (Utilities|Array|IsValidIndex _quests)
        (Variables|Default|SetAvailableQuest (Utilities|Array|Get(acopy) _quests))
        ;[1 0 0.06701] And remove it from array
        (Utilities|Array|RemoveIndex (Variables|Default|GetQuests))
        ;[1 1 1] Ending interaction
        (Class|BaseInteractionActor|OnInteractionFinished (Variables|Default|GetQuest_Instigator))
        (Variables|Default|SetQuest_Instigator 0)
        (else
          ;[1 0 0.07575] Clear Available Quest var if all quests have been taken
          (Variables|Default|SetAvailableQuest 0)
          (Class|BaseInteractionActor|OnInteractionFinished (Variables|Default|GetQuest_Instigator))
          (Variables|Default|SetQuest_Instigator 0))))
    (:else
      (Class|BaseInteractionActor|OnInteractionFinished (Variables|Default|GetQuest_Instigator))
      (Development|PrintString "No quests available" true true "(R=0.000000,G=1.000000,B=0.332829,A=1.000000)" 3.0)
      (Variables|Default|SetQuest_Instigator 0))))

(fn ConstructionScript)