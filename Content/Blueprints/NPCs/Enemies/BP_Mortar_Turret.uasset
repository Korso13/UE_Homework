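; BP_Mortar_Turret is an enemy mortar turret Blueprint that shows its health on a 3D HP bar widget.
; On BeginPlay it runs the parent logic, caches the bar as W_EnemyHPBar and fills it from HealthComponent's current and max HP.
; The OnTakingDamage event pushes updated values to the bar.
; No firing or targeting logic appears in this graph.
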(event EventBeginPlay
  (bind _healthcomponent (Variables|Default|GetHealthComponent))
  ;[1 1 1] Initial HP Bar setup
  (|CallParentFunction)
  (bind _asw_enemy_hpbar (Utilities|Casting|CastToW_EnemyHPBar (UserInterface|GetWidget (Variables|Default|Get3D_HP_bar))))
  (Default|HPBarChange _asw_enemy_hpbar _asw_enemy_hpbar (Variables|/Script/Tankogeddon.HealthComponent|GetCurrentHP _healthcomponent) (Variables|/Script/Tankogeddon.HealthComponent|GetMaxHP _healthcomponent)))

(event Collision|EventActorBeginOverlap
  (params (OtherActor :type Actor%20Object%20Reference))
  (|CallParentFunction OtherActor) ; This node is disabled and will not be called.\nDrag off pins to build functionality.
)

(event EventTick
  (params (DeltaSeconds :type Float%20%28single-precision%29))
  (|CallParentFunction DeltaSeconds) ; This node is disabled and will not be called.\nDrag off pins to build functionality.
)

(event EventOnTakingDamage
  (params (Damage :type Damage%20Info%20Structure))
  (bind _healthcomponent (Variables|Default|GetHealthComponent))
  ;[1 1 1] Binding Damage Event to change HP bar
  (Default|HPBarChange (stale EventBeginPlay _asw_enemy_hpbar) (stale EventBeginPlay _asw_enemy_hpbar) (Variables|/Script/Tankogeddon.HealthComponent|GetCurrentHP _healthcomponent) (Variables|/Script/Tankogeddon.HealthComponent|GetMaxHP _healthcomponent)))

(fn ConstructionScript
  (|CallParentFunction))