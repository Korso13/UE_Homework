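; SatelliteStation is an interactable quest giver that hands a single available quest to whoever interacts with it.
; On Interact it attaches the quest actor to the instigator, prints a greeting and the quest description, then calls TakeQuest.
; It then clears its quest reference, so later interactions only report that the interaction finished.
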(event EventBeginPlay)

(event Collision|EventActorBeginOverlap
  (params (OtherActor :type Actor%20Object%20Reference)))

(event EventTick
  (params (DeltaSeconds :type Float%20%28single-precision%29)))

(event EventInteract
  (params (Instigator :type Actor%20Object%20Reference))
  (Variables|Default|SetQuest_Instigator Instigator)
  (bind _availablequest (Variables|Default|GetAvailableQuest)
    (:then
      (Transformation|AttachActorToActor _availablequest (Variables|Default|GetQuest_Instigator) "None" "SnapToTarget" "SnapToTarget" "SnapToTarget" true)
      (Development|PrintString (Utilities|String|Append "Hello,  " (Utilities|GetDisplayName (Variables|Default|GetQuest_Instigator)) "! Here is your mission!") true true "(R=0.000000,G=0.660000,B=1.000000,A=1.000000)" 3.0)
      (Development|PrintString (Utilities|String|ToString(Text) (Variables|/Script/QuestSystem.Quest|GetQuestDescription (Variables|Default|GetAvailableQuest))) true true "(R=0.000000,G=1.000000,B=0.172531,A=1.000000)" 7.0)
      (Class|Quest|TakeQuest (Variables|Default|GetAvailableQuest) (Variables|Default|GetQuest_Instigator))
      (Variables|Default|SetAvailableQuest 0)
      (Class|BaseInteractionActor|OnInteractionFinished (Variables|Default|GetQuest_Instigator))
      (Variables|Default|SetQuest_Instigator 0))
    (:else
      (Class|BaseInteractionActor|OnInteractionFinished (Variables|Default|GetQuest_Instigator)))))

(fn ConstructionScript)