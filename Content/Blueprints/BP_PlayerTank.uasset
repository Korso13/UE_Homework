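; BP_PlayerTank is the player tank Blueprint, handling the status HUD and game-over screen.
; On BeginPlay it shows the player status widget through HUD_Manager, plays that widget's HUDLoad animation and caches the player pawn.
; When destroyed, it checks IsKIA on the cached pawn and, if true, swaps the status widget for the game-over widget.
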(event EventBeginPlay
  ;[1 1 1] Player HUD init
  (bind _ashud_manager (Utilities|Casting|CastToHUD_Manager (HUD|GetHUD (Game|GetPlayerController 0))))
  (bind _output_get (Variables|Default|SetAs%20HUD%20Manager _ashud_manager))
  (bind _returnvalue (Class|HUDManager|ShowWidget _output_get "Widget_PlayerStatus"))
  (bind _asw_player_status (Utilities|Casting|CastToW_PlayerStatus _returnvalue))
  ;[1 1 1] Player HUD load anim
  (UserInterface|Animation|PlayAnimation _asw_player_status (Variables|/Game/Widgets/W_PlayerStatus.W_PlayerStatus_C|GetHUD_load _asw_player_status) 0.0 1 "Forward" 1.0 false)
  ;[1 1 1] Game over sign call
  (bind _output_get_2 (Variables|Default|SetNewVar_1 (Game|Player|GetPlayerPawn 0))))

(event Collision|EventActorBeginOverlap
  (params (OtherActor :type Actor%20Object%20Reference)))

(event EventTick
  (params (DeltaSeconds :type Float%20%28single-precision%29)))

(event EventDestroyed
  ;[1 1 1] Game over sign call
  (bind _asbp_player_tank (Utilities|Casting|CastToBP_PlayerTank (stale EventBeginPlay _output_get_2)))
  (if (Class|BasePawn|IsKIA _asbp_player_tank)
    (Class|HUDManager|HideWidget (stale EventBeginPlay _output_get) "Widget_PlayerStatus")
    (Class|HUDManager|ShowWidget (stale EventBeginPlay _output_get) "Widget_GameOver")))

(fn ConstructionScript)